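; Extraction point actor that detects players entering and leaving a resizable box and notifies them through interface messages.
; On the server, box overlap records actors of allowed classes and, if they support this named location, starts their extraction countdown, otherwise shows a denied widget.
; A looping server timer, rather than end overlap, compares overlaps against that list to clear departed players' extraction status.
; Clients only set the location name text.
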(event OnComponentBeginOverlap(Box)
  (params (OverlappedComponent :type Primitive%20Component%20Object%20Reference) (OtherActor :type Actor%20Object%20Reference) (OtherComp :type Primitive%20Component%20Object%20Reference) (OtherBodyIndex :type Integer) (bFromSweep :type Boolean) (SweepResult :type Hit%20Result%20Structure%20%28by%20ref%29))
  (bind _actorsextracting (Variables|Default|GetActorsExtracting))
  ;[1 1 1] All this actor needs to do is detect when the player goes inside the collision (extract) zone and when they leave it. Both events trigger interface events on the player.
  (Networking|SwitchHasAuthority
    (:Authority
      (if (and (not (Utilities|Array|ContainsItem _actorsextracting OtherActor)) (Utilities|Array|ContainsItem (Variables|Default|GetExtractClassTypes) (Utilities|GetClass OtherActor)))
        (Utilities|Array|AddUnique _actorsextracting OtherActor)
        (bind _isvalidextraction (Class|ExtractionInterface|DetectSupportedExtractLocaiton(Message) OtherActor (Variables|Default|GetExtractLocationName)))
        (if _isvalidextraction
          (Class|ExtractionInterface|StartExtractionCountdown(Message) OtherActor)
          (Class|ExtractionInterface|UpdatePlayerExtractionStatus(Message) OtherActor true)
          (else
            (Class|ExtractionInterface|CreateExtractionDeniedWidget(Message) OtherActor)))))))

(event OnComponentEndOverlap(Box)
  (params (OverlappedComponent :type Primitive%20Component%20Object%20Reference) (OtherActor :type Actor%20Object%20Reference) (OtherComp :type Primitive%20Component%20Object%20Reference) (OtherBodyIndex :type Integer))
  ;[1 1 1] All this actor needs to do is detect when the player goes inside the collision (extract) zone and when they leave it. Both events trigger interface events on the player.
)

(event Custom|SERVER_MonitorExtractionZone
  ;[1 1 1] All this actor needs to do is detect when the player goes inside the collision (extract) zone and when they leave it. Both events trigger interface events on the player.
  (if (not (Class|KismetSystemLibrary|TimerExistsHandle (Variables|Default|GetPlayerExtractionTimerHandle)))
    (bind _returnvalue (Utilities|Time|SetTimerbyEvent (delegate Custom|TimerEvent_DetectPlayersInExtractionZone) 0.2 true))
    (Variables|Default|SetPlayerExtractionTimerHandle _returnvalue)))

(event Custom|TimerEvent_DetectPlayersInExtractionZone
  (bind _box (Variables|Default|GetBox))
  (bind _actorsextracting (Variables|Default|GetActorsExtracting))
  (bind _overlappingactors (Collision|GetOverlappingActors _box "/Game/Extraction/Blueprints/Character/FirstPersonCharacter.FirstPersonCharacter_C" :!class /Script/Engine.PrimitiveComponent))
  ;[1 1 1] All this actor needs to do is detect when the player goes inside the collision (extract) zone and when they leave it. Both events trigger interface events on the player.
  (if (not (Utilities|Array|Identical _overlappingactors (Variables|Default|GetActorsExtracting)))
    (for _array_element _actorsextracting
      (if (not (Utilities|Array|ContainsItem _overlappingactors _array_element))
        (Class|ExtractionInterface|UpdatePlayerExtractionStatus(Message) _array_element false)
        (Utilities|Array|RemoveItem _actorsextracting _array_element)))))

(event EventBeginPlay
  (Utilities|FlowControl|Delay 0.2)
  (Networking|SwitchHasAuthority
    (:Authority
      (CallFunction|SERVERMonitorExtractionZone))
    (:Remote
      (Rendering|Components|TextRender|SetText (Variables|Default|GetTextRender) (Utilities|Text|ToText(String) (Utilities|String|Append "Extraction Location: " (Utilities|String|EnumtoString (Variables|Default|GetExtractLocationName))))))))

(fn ConstructionScript
  (Components|Box|SetBoxExtent (Variables|Default|GetBox) (Variables|Default|GetExtractCollisionBoxSize) true))