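; Actor component that manages extraction for its owning player actor: assigned locations, countdown and related client widgets.
; On BeginPlay the authority picks one random location from Alpha to Delta; client events display and highlight assigned locations.
; A looping server timer accumulates time inside the zone, resetting on exit.
; On completion it shows the success widget and destroys the owner; stats and inventory persistence are only print-string placeholders.
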(event Custom|CLIENT_CreateExtractionWidget
  (bind _returnvalue (UserInterface|CreateWidget "/Game/Extraction/Widgets/ExtractionCountdown.ExtractionCountdown_C"))
  (bind _output_get (Variables|Default|SetExtractionWidget _returnvalue))
  (UserInterface|Viewport|AddtoViewport _output_get 0))

(event Custom|CLIENT_CreateExtractionSuccessWidget
  (bind _returnvalue (UserInterface|CreateWidget "/Game/Extraction/Widgets/ExtractionSuccess.ExtractionSuccess_C"))
  (bind _output_get (Variables|Default|SetExtractionSuccessWidget _returnvalue))
  (UserInterface|Viewport|AddtoViewport _output_get 0))

(event Custom|SERVER_SetPlayerExtractionLocations
  (params (Selection :type Array%20of%20ExtractionLocationNames%20Enums :default "NewEnumerator0") (Random :type Boolean))
  (bind _returnvalue (Math|Random|RandomIntegerinRange -9128 9128))
  (bind _returnvalue_2 (Math|Random|MakeRandomStream _returnvalue))
  (bind _returnvalue_3 (Class|KismetMathLibrary|RandomIntegerfromStream 3 _returnvalue_2))
  (if Random
    (switch int _returnvalue_3
      (:0
        (Utilities|Array|AddUnique (Variables|Default|GetAvailableExtractionLocations) "NewEnumerator0" :!label _label))
      (:1
        (Utilities|Array|AddUnique (Variables|Default|GetAvailableExtractionLocations) "NewEnumerator1" :!label _label_2))
      (:2
        (Utilities|Array|AddUnique (Variables|Default|GetAvailableExtractionLocations) "NewEnumerator2" :!label _label_3))
      (:3
        (Utilities|Array|AddUnique (Variables|Default|GetAvailableExtractionLocations) "NewEnumerator3" :!label _label_4)))
    (else
      (for _array_element Selection
        (switch Utilities|FlowControl|Switch|SwitchonExtractionLocationNames (select Random (Utilities|Enum|LiteralenumExtractionLocationNames (Utilities|Enum|ByteToEnumExtractionLocationNames (Math|Conversions|ToByte(Integer) _returnvalue_3))) _array_element)
          (:NewEnumerator0
            (goto _label))
          (:NewEnumerator1
            (goto _label_2))
          (:NewEnumerator2
            (goto _label_3))
          (:NewEnumerator3
            (goto _label_4)))))))

(event Custom|CLIENT_ToggleTextColor
  (params (ExtractLocation :type ExtractionLocationNames%20Enum :default "NewEnumerator0"))
  (bind _newvar_0 (Variables|Default|GetNewVar_0))
  (Utilities|IsValid _newvar_0
    (:Is%20Valid
      (Default|CLIENTToggleBorderColor _newvar_0 ExtractLocation))))

(event Custom|CLIENT_CreateInvalidExtractionWidget
  (bind _returnvalue (UserInterface|CreateWidget "/Game/Extraction/Widgets/InvalidExtractLocation.InvalidExtractLocation_C"))
  (UserInterface|Viewport|AddtoViewport _returnvalue 0))

(event Custom|SERVER_CreateExtractionLocationsWidget
  (CallFunction|CLIENTCreateExtractionLocationsWidget (Variables|Default|GetAvailableExtractionLocations)))

(event Custom|CLIENT_PulseExtractLocationText
  (params (Location :type ExtractionLocationNames%20Enum :default "NewEnumerator0"))
  (Default|PlayPulseTextAnimation (Variables|Default|GetNewVar_0) Location))

(event Custom|CLIENT_CreateExtractFailedWidget
  (bind _returnvalue (UserInterface|CreateWidget "/Game/Extraction/Widgets/FailedToExtractWidget.FailedToExtractWidget_C"))
  (UserInterface|Viewport|AddtoViewport _returnvalue 0))

(event Custom|CLIENT_DestroyExtractionTimerWidget
  (bind _extractionwidget (Variables|Default|GetExtractionWidget))
  (Utilities|IsValid _extractionwidget
    (:Is%20Valid
      (Widget|RemovefromParent _extractionwidget))))

(event Custom|SERVER_StartExtractionCountdown
  (params (ExtractedActor :type Actor%20Object%20Reference))
  (if (not (Class|KismetSystemLibrary|TimerExistsHandle (Variables|Default|GetPlayerExtractionTimerHandle)))
    (Class|ExtractionInterface|CreateExtractionWidget(Message) ExtractedActor)
    (bind _returnvalue (Utilities|Time|SetTimerbyEvent (delegate Custom|TimerEvent_ExtractPlayer) 0.2 true))
    (Variables|Default|SetPlayerExtractionTimerHandle _returnvalue)
    (CallFunction|CLIENTPulseExtractLocationText (Utilities|Array|Get(acopy) (Variables|Default|GetAvailableExtractionLocations)))))

(event Custom|TimerEvent_ExtractPlayer
  (if (Variables|Default|GetisPlayerInExtractionZone)
    (bind _output_get (Variables|Default|SetCurrentExtractTimeSeconds (+ (Variables|Default|GetCurrentExtractTimeSeconds) 0.2)))
    (if (>= _output_get (Variables|Default|GetMaxExtractTimeSeconds))
      (Development|PrintString "Extraction Successful, Extracting Player...")
      (Variables|Default|SetCurrentExtractTimeSeconds 0.0)
      (CallFunction|CLIENTCreateExtractionSuccessWidget)
      (Utilities|Time|ClearandInvalidateTimerbyHandle (Variables|Default|GetPlayerExtractionTimerHandle))
      (CallFunction|SERVERHandlePostExtractionEvent)
      (else
        (Development|PrintString "Keep waiting for extract timer...")))
    (else
      (Development|PrintString "Player left the extraction zone, resetting...")
      (Class|ExtractionInterface|DestroyExtractionWidget(Message) (stale Custom|SERVER_StartExtractionCountdown ExtractedActor))
      (Variables|Default|SetCurrentExtractTimeSeconds 0.0)
      (Utilities|Time|ClearandInvalidateTimerbyHandle (Variables|Default|GetPlayerExtractionTimerHandle))
      (Utilities|Array|RemoveItem (Variables|Default|GetActorsExtracting) (stale Custom|SERVER_StartExtractionCountdown ExtractedActor)))))

(event Custom|SERVER_ResetExtraction
  (bind _extractionsuccesswidget (Variables|Default|GetExtractionSuccessWidget))
  (bind _playerextractiontimerhandle (Variables|Default|GetPlayerExtractionTimerHandle))
  (bind _extractionwidget (Variables|Default|GetExtractionWidget))
  (Variables|Default|SetisPlayerInExtractionZone false)
  (Variables|Default|SetCurrentExtractTimeSeconds 0.0)
  (Utilities|FlowControl|Sequence
    (:then_0
      (if (Utilities|Time|IsValidTimerHandle _playerextractiontimerhandle)
        (Utilities|Time|ClearandInvalidateTimerbyHandle _playerextractiontimerhandle)))
    (:then_1
      (Utilities|IsValid _extractionwidget
        (:Is%20Valid
          (Widget|RemovefromParent _extractionwidget))))
    (:then_2
      (Utilities|IsValid _extractionsuccesswidget
        (:Is%20Valid
          (Widget|RemovefromParent _extractionsuccesswidget))))))

(event Custom|CLIENT_CreateExtractionLocationsWidget
  (params (Locations :type Array%20of%20ExtractionLocationNames%20Enums :default "NewEnumerator0"))
  (bind _returnvalue (UserInterface|CreateWidget "/Game/Extraction/Widgets/ExtractionPointsWidget1.ExtractionPointsWidget1_C"))
  (bind _output_get (Variables|Default|SetNewVar_0 _returnvalue))
  (Utilities|FlowControl|Delay 2.0)
  (UserInterface|Viewport|AddtoViewport _output_get 0)
  (for _array_element Locations
    (Default|CLIENTToggleBorderColor _output_get _array_element)))

(event Custom|CLIENT_ShowExtractionLocationsWidget
  (Utilities|FlowControl|DoOnce false :!label _label
    (:Completed
      (Default|PlayWidgetAnimation (Variables|Default|GetNewVar_0))
      (Utilities|FlowControl|Delay 6.0)
      (goto _label Reset))))

(event Custom|SERVER_HandlePostExtractionEvent
  (Actor|DestroyActor (Components|GetOwner))
  (Development|PrintString "Updating Account Records With Stats....")
  (Development|PrintString "Adding Inventory Items To Persistent DB"))

(event EventBeginPlay
  (if (Ability|HasAuthority (Components|GetOwner))
    (CallFunction|SERVERSetPlayerExtractionLocations (Utilities|Array|MakeArray "NewEnumerator0" "NewEnumerator3") true)
    (for _array_element (Variables|Default|GetAvailableExtractionLocations)
      (CallFunction|CLIENTToggleTextColor _array_element))))

(fn SetRandomExtractionLocations
  (bind _returnvalue (Utilities|Array|AddUnique (Variables|Default|GetAvailableExtractionLocations) (Utilities|Enum|LiteralenumExtractionLocationNames (Utilities|Enum|ByteToEnumExtractionLocationNames (Math|Conversions|ToByte(Integer) (Math|Random|RandomInteger 3))))))
  (return (!= _returnvalue -1)))