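; Player controller for the Extraction game that relays level load and respawn requests through server and client events.
; The client respawn event passes the controlled pawn to the server event, which acts only if that pawn is invalid.
; It then asks ExtractionGameMode to respawn this controller as a FirstPersonCharacter.
; A separate server event opens a level by name.
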(event Custom|CLIENT_RespawnPlayer
  (CallFunction|SERVERRespawnPlayer (Pawn|GetControlledPawn self)))

(event Custom|SERVER_RespawnPlayer
  (params (PlayerPawn :type Pawn%20Object%20Reference))
  (bind _returnvalue (Game|GetGameMode))
  (Utilities|IsValid PlayerPawn
    (:Is%20Not%20Valid
      (Utilities|IsValid _returnvalue
        (:Is%20Valid
          (bind _asextraction_game_mode (Utilities|Casting|CastToExtractionGameMode _returnvalue))
          (Default|SERVERRespawn _asextraction_game_mode self "/Game/Extraction/Blueprints/Character/FirstPersonCharacter.FirstPersonCharacter_C"))))))

(event Custom|SERVER_LoadLevel
  (params (LevelName :type Name))
  (Game|OpenLevel(byName) LevelName))

(fn ConstructionScript)